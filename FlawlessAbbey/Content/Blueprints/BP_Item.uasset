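; BP_Item is a world item that the player can pick up into an inventory.
; On BeginPlay it binds overlap events on its sphere component to show a pickup prompt widget, given the item and pawn, while BP_ThirdPersonCharacter is in range.
; StartInteraction calls PickUp, which passes the item itself to the BPC_Inventory component on player 0's pawn.
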(event `self.ReceiveBeginPlay`
  (bind _returnvalue (`self.GetComponentByClass` "/Script/Engine.SphereComponent"))
  (`/Engine/EditorBlueprintResources/StandardMacros.IsValid` _returnvalue
    (:`Is Valid`
      (add `PrimitiveComponent.OnComponentBeginOverlap` _returnvalue (`|CreateDelegate` :!event `OnComponentBeginOverlap`))
      (add `PrimitiveComponent.OnComponentEndOverlap` _returnvalue (`|CreateDelegate` :!event `OnComponentEndOverlap`)))))

(event `/Game/Blueprints/Interface/BPI_Interact.StartInteraction`
  (`self.PickUp`))

(fn `OnComponentBeginOverlap`
  (params (OverlappedComponent :type "PrimitiveComponent Object Reference") (OtherActor :type "Actor Object Reference") (OtherComp :type "PrimitiveComponent Object Reference") (OtherBodyIndex :type Integer) (bFromSweep :type Boolean) (SweepResult :type "HitResult Structure (by ref)"))
  (bind _asbp_third_person_character (cast `/Game/ThirdPerson/Blueprints/BP_ThirdPersonCharacter` OtherActor))
  (bind _returnvalue (`|CreateWidget` "/Game/Blueprints/UI/WBP_PickupPrompt.WBP_PickupPrompt_C" null self _asbp_third_person_character))
  (set `self.PickupPromptWidget` _returnvalue)
  (`UserWidget.AddToViewport` (`self.PickupPromptWidget`) 0)
  (return))

(fn `OnComponentEndOverlap`
  (params (OverlappedComponent :type "PrimitiveComponent Object Reference") (OtherActor :type "Actor Object Reference") (OtherComp :type "PrimitiveComponent Object Reference") (OtherBodyIndex :type Integer))
  (cast `/Game/ThirdPerson/Blueprints/BP_ThirdPersonCharacter` OtherActor)
  (`Widget.RemoveFromParent` (`self.PickupPromptWidget`)))

(fn `PickUp`
  (locals (InventoryComponent :type "/Game/Blueprints/Components/BPC_Inventory Object Reference"))
  (set `local.InventoryComponent` (`self.GetComponentByClass` (`Controller.K2_GetPawn` (`GameplayStatics.GetPlayerController` 0)) "/Game/Blueprints/Components/BPC_Inventory.BPC_Inventory_C"))
  (`/Game/Blueprints/Components/BPC_Inventory.AddToInventory` (`local.InventoryComponent`) self))

(fn `PresentPickUpPrompt`
  (params (OverlappedComponent :type "PrimitiveComponent Object Reference") (OtherActor :type "Actor Object Reference") (OtherComp :type "PrimitiveComponent Object Reference") (OtherBodyIndex :type Integer) (bFromSweep :type Boolean) (SweepResult :type "HitResult Structure (by ref)"))
  (cast `/Game/ThirdPerson/Blueprints/BP_ThirdPersonCharacter` OtherActor)
  (bind _returnvalue (`|CreateWidget` "/Game/Blueprints/UI/WBP_PickupPrompt.WBP_PickupPrompt_C" null null null))
  (`UserWidget.AddToViewport` _returnvalue 0)
  (return))

(fn `UserConstructionScript`)