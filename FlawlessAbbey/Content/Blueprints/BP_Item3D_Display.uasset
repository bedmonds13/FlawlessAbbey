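; BP_Item3D_Display is an actor that shows a 3D item mesh through a scene capture, with player-controlled rotation.
; On BeginPlay, its SceneCaptureComponent2D is restricted to show only the StaticMesh component, isolating it in the capture.
; Each tick polls Q and E on player controller 0 to yaw the mesh in opposite directions by a fixed per-frame step, unscaled by delta time.
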(event `self.ReceiveBeginPlay`
  (`SceneCaptureComponent.ShowOnlyComponent` (`self.SceneCaptureComponent2D`) (`self.StaticMesh`)))

(event `self.ReceiveTick`
  (params (DeltaSeconds :type "Float (single-precision)"))
  (bind _returnvalue (`GameplayStatics.GetPlayerController` 0))
  (`SceneComponent.K2_AddLocalRotation` (`self.StaticMesh`) (`KismetMathLibrary.MakeRotator` 0.0 0.0 (+ (`KismetMathLibrary.SelectFloat` 1.0 0.0 (`PlayerController.IsInputKeyDown` _returnvalue "Q")) (`KismetMathLibrary.SelectFloat` -1.0 0.0 (`PlayerController.IsInputKeyDown` _returnvalue "E")))) false false))

(fn `UserConstructionScript`)