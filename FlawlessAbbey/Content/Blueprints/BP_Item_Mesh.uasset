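; BP_Item_Mesh is an item actor that displays a configurable static mesh as a physics-simulated object.
; The construction script runs the parent's logic, then assigns the Mesh variable to the StaticMesh component.
; BeginPlay calls the parent, then enables physics simulation on the component only if it holds a valid mesh.
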(event `self.ReceiveBeginPlay`
  (`parent.ReceiveBeginPlay`)
  (`/Engine/EditorBlueprintResources/StandardMacros.IsValid` (`StaticMeshComponent.StaticMesh` (`self.StaticMesh`))
    (:`Is Valid`
      (`PrimitiveComponent.SetSimulatePhysics` (`self.StaticMesh`) true))))

(fn `UserConstructionScript`
  (`parent.UserConstructionScript`)
  (`StaticMeshComponent.SetStaticMesh` (`self.StaticMesh`) (`self.Mesh`)))