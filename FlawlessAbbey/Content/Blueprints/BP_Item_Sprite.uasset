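; BP_Item_Sprite is an item actor that displays a Paper2D sprite turned to face the player camera.
; The construction script calls its parent, then applies the Sprite variable to the PaperSprite component.
; Each Tick computes a look-at from the root's relative transform to player 0's camera location.
; Only the yaw is used, offset by a quarter turn, so the sprite billboards around the vertical axis and stays upright.
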(event `self.ReceiveTick`
  (params (DeltaSeconds :type "Float (single-precision)"))
  (bind (_returnvalue_roll _returnvalue_pitch _returnvalue_yaw) (`KismetMathLibrary.BreakRotator` (`KismetMathLibrary.FindRelativeLookAtRotation` (`SceneComponent.GetRelativeTransform` (`self.DefaultSceneRoot`)) (`PlayerCameraManager.GetCameraLocation` (`PlayerController.PlayerCameraManager` (`GameplayStatics.GetPlayerController` 0))))))
  (`SceneComponent.K2_SetRelativeRotation` (`self.PaperSprite`) (`KismetMathLibrary.MakeRotator` 0.0 0.0 (+ _returnvalue_yaw 90.0)) false false))

(fn `UserConstructionScript`
  (`parent.UserConstructionScript`)
  (`PaperSpriteComponent.SetSprite` (`self.PaperSprite`) (`self.Sprite`)))