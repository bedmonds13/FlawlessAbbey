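; BP_Interactible is a world actor the player can interact with to open a dialogue.
; Its box overlap with BP_ThirdPersonCharacter creates a WBP_PickupPrompt widget, passing itself and the pawn, and removes it when the overlap ends.
; The StartInteraction event creates a WBP_DialogueBox from the actor's DialogueSequence and adds it to the viewport.
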(event `/Game/Blueprints/Interface/BPI_Interact.StartInteraction`
  (bind _returnvalue (`|CreateWidget` "/Game/Blueprints/UI/WBP_DialogueBox.WBP_DialogueBox_C" null (`self.Dialogue Sequence`)))
  (`UserWidget.AddToViewport` _returnvalue 0))

(event `self.Box.OnComponentBeginOverlap`
  (params (OverlappedComponent :type "PrimitiveComponent Object Reference") (OtherActor :type "Actor Object Reference") (OtherComp :type "PrimitiveComponent Object Reference") (OtherBodyIndex :type Integer) (bFromSweep :type Boolean) (SweepResult :type "HitResult Structure (by ref)"))
  (bind _asbp_third_person_character (cast `/Game/ThirdPerson/Blueprints/BP_ThirdPersonCharacter` OtherActor))
  (bind _returnvalue (`|CreateWidget` "/Game/Blueprints/UI/WBP_PickupPrompt.WBP_PickupPrompt_C" null self _asbp_third_person_character))
  (set `self.PickupPromptWidget` _returnvalue)
  (`UserWidget.AddToViewport` (`self.PickupPromptWidget`) 0))

(event `self.Box.OnComponentEndOverlap`
  (params (OverlappedComponent :type "PrimitiveComponent Object Reference") (OtherActor :type "Actor Object Reference") (OtherComp :type "PrimitiveComponent Object Reference") (OtherBodyIndex :type Integer))
  (cast `/Game/ThirdPerson/Blueprints/BP_ThirdPersonCharacter` OtherActor)
  (`Widget.RemoveFromParent` (`self.PickupPromptWidget`)))

(fn `UserConstructionScript`)